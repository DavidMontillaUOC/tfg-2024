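; Base player controller that owns the player's HUD and character stat menu and relays stat changes to both.
; BeginPlay creates both widgets and adds them to the viewport, with the stat menu starting hidden.
; HP and stamina events update the HUD bars plus truncated integer text in the menu.
; Separate events write attributes (Spanish-named), level, experience and attribute points straight into the menu's text blocks.
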(event Custom|UpdateStamina
  (params (CurrentStamina :type Float%20%28double-precision%29) (MaxStamina :type Float%20%28double-precision%29))
  (Default|SetStaminaBar (Variables|Default|GetUI) CurrentStamina MaxStamina)
  (Rendering|Components|TextRender|SetText (Variables|/Game/UI/StatMenu.StatMenu_C|GetTextStamina (Variables|Default|GetStatMenu)) (Utilities|Text|ToText(Integer) (Math|Float|Truncate MaxStamina))))

(event Custom|UpdateAgi
  (params (SabValue :type Integer))
  (Rendering|Components|TextRender|SetText (Variables|/Game/UI/StatMenu.StatMenu_C|GetTextAgilidad (Variables|Default|GetStatMenu)) (Utilities|Text|ToText(Integer) SabValue)))

(event Custom|UpdateFue
  (params (FueValue :type Integer))
  (Rendering|Components|TextRender|SetText (Variables|/Game/UI/StatMenu.StatMenu_C|GetTextFuerza (Variables|Default|GetStatMenu)) (Utilities|Text|ToText(Integer) FueValue)))

(event Custom|UpdateEnergia
  (params (EnePoints :type Integer))
  (Rendering|Components|TextRender|SetText (Variables|/Game/UI/StatMenu.StatMenu_C|GetTextEnergia (Variables|Default|GetStatMenu)) (Utilities|Text|ToText(Integer) EnePoints)))

(event Custom|UpdateLevel
  (params (LvlValue :type Integer))
  (Rendering|Components|TextRender|SetText (Variables|/Game/UI/StatMenu.StatMenu_C|GettextLvl (Variables|Default|GetStatMenu)) (Utilities|Text|ToText(Integer) LvlValue)))

(event Custom|UpdateAttributePoints
  (params (AttPoints :type Integer))
  (Rendering|Components|TextRender|SetText (Variables|/Game/UI/StatMenu.StatMenu_C|GetTextPuntosHabilidad (Variables|Default|GetStatMenu)) (Utilities|Text|ToText(Integer) AttPoints)))

(event Custom|UpdateHP
  (params (CurrentHP :type Float%20%28double-precision%29) (MaxHP :type Float%20%28double-precision%29))
  (Default|SetHPBar (Variables|Default|GetUI) CurrentHP MaxHP)
  (Rendering|Components|TextRender|SetText (Variables|/Game/UI/StatMenu.StatMenu_C|GetTextMaxHealth (Variables|Default|GetStatMenu)) (Utilities|Text|ToText(Integer) (Math|Float|Truncate MaxHP)))
  (Rendering|Components|TextRender|SetText (Variables|/Game/UI/StatMenu.StatMenu_C|GetTextCurrentHealth (Variables|Default|GetStatMenu)) (Utilities|Text|ToText(Integer) (Math|Float|Truncate CurrentHP))))

(event Custom|UpdateExp
  (params (CurrentEXP :type Integer) (NeededEXP :type Integer))
  (bind _statmenu (Variables|Default|GetStatMenu))
  (Rendering|Components|TextRender|SetText (Variables|/Game/UI/StatMenu.StatMenu_C|GettextCurrentExp _statmenu) (Utilities|Text|ToText(Integer) CurrentEXP))
  (Rendering|Components|TextRender|SetText (Variables|/Game/UI/StatMenu.StatMenu_C|GetTextExpNeeded _statmenu) (Utilities|Text|ToText(Integer) NeededEXP)))

(event Custom|UpdateVitalidad
  (params (VitValue :type Integer))
  (Rendering|Components|TextRender|SetText (Variables|/Game/UI/StatMenu.StatMenu_C|GetTextVitalidad (Variables|Default|GetStatMenu)) (Utilities|Text|ToText(Integer) VitValue)))

(event Custom|UpdateSabiduria
  (params (SabValue :type Integer))
  (Rendering|Components|TextRender|SetText (Variables|/Game/UI/StatMenu.StatMenu_C|GetTextSabiduria (Variables|Default|GetStatMenu)) (Utilities|Text|ToText(Integer) SabValue)))

(event Custom|UpdateInt
  (params (IntValue :type Integer))
  (Rendering|Components|TextRender|SetText (Variables|/Game/UI/StatMenu.StatMenu_C|GetTextInteligencia (Variables|Default|GetStatMenu)) (Utilities|Text|ToText(Integer) IntValue)))

(event EventBeginPlay
  (bind _returnvalue (UserInterface|CreateWidget "/Game/UI/inGameUI.inGameUI_C"))
  (bind _output_get (Variables|Default|SetUI _returnvalue))
  (UserInterface|Viewport|AddtoViewport _output_get 0)
  (bind _returnvalue_2 (UserInterface|CreateWidget "/Game/UI/StatMenu.StatMenu_C"))
  (bind _output_get_2 (Variables|Default|SetStatMenu _returnvalue_2))
  (UserInterface|Viewport|AddtoViewport _output_get_2 0)
  (Widget|SetVisibility _output_get_2 "Hidden"))

(fn ConstructionScript)