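; Boss enemy character that detects the top-down player through a sphere overlap, then pursues and shoots at them.
; Tick runs the chase, which disables movement at close range, and a cooldown-gated burst of magic projectiles aimed at the player via RapidFire and Shot.
; At half health or below it enrages, adding a second burst to each attack.
; Damage spawns floating numbers, and death grants the player EXP.
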(event OnComponentBeginOverlap(Sphere)
  (params (OverlappedComponent :type Primitive%20Component%20Object%20Reference) (OtherActor :type Actor%20Object%20Reference) (OtherComp :type Primitive%20Component%20Object%20Reference) (OtherBodyIndex :type Integer) (bFromSweep :type Boolean) (SweepResult :type Hit%20Result%20Structure%20%28by%20ref%29))
  (Utilities|Casting|CastToTopDownCharacterBlueprint OtherActor)
  (Variables|Default|SetseesPlayer true))

(event OnComponentEndOverlap(Sphere)
  (params (OverlappedComponent :type Primitive%20Component%20Object%20Reference) (OtherActor :type Actor%20Object%20Reference) (OtherComp :type Primitive%20Component%20Object%20Reference) (OtherBodyIndex :type Integer))
  (Utilities|Casting|CastToTopDownCharacterBlueprint OtherActor)
  (Variables|Default|SetseesPlayer false))

(event Custom|ShotPlayer
  (if (and (Variables|Default|GetseesPlayer) (not (Variables|Default|GetisShooting)))
    (Variables|Default|SetisShooting true)
    (|RapidFire)
    (if (Variables|Default|Getenrage)
      (|RapidFire_2))
    (Utilities|FlowControl|Delay 2.0)
    (Variables|Default|SetisShooting false)))

(event Custom|FollowPlayer
  (bind (_returnvalue_x _returnvalue_y) (|ReturnPlayerDirection_2))
  ;[1 1 1] Track Player
  (if (Variables|Default|GetseesPlayer)
    (if (> (Math|Vector|VectorLength (Math|Vector|MakeVector _returnvalue_x _returnvalue_y 0.0)) 1.2e+02)
      (Pawn|Components|CharacterMovement|SetMovementMode (Variables|Character|GetCharacterMovement) "MOVE_None" 0)
      (Pawn|Input|AddMovementInput (Math|Vector|MakeVector _returnvalue_x 0.0 0.0) 1.0 false)
      (Pawn|Input|AddMovementInput (Math|Vector|MakeVector 0.0 _returnvalue_y 0.0) 1.0 false)
      (Variables|Default|SetDirection (Math|Vector2D|MakeVector2D _returnvalue_x _returnvalue_y))
      (Variables|Default|SetcanAttack false)
      (else
        (Pawn|Components|CharacterMovement|DisableMovement (Variables|Character|GetCharacterMovement))
        (Variables|Default|SetcanAttack true)))))

(event EventBeginPlay
  (Variables|Default|SetseesPlayer false)
  (Variables|Default|SetCurrentEnemyHP (Variables|Default|GetMaxEnemyHP)))

(event Collision|EventActorBeginOverlap
  (params (OtherActor :type Actor%20Object%20Reference)))

(event EventTick
  (params (DeltaSeconds :type Float%20%28single-precision%29))
  (if (<= (Variables|Default|GetCurrentEnemyHP) (/ (Variables|Default|GetMaxEnemyHP) 2))
    (Variables|Default|Setenrage true))
  (CallFunction|ShotPlayer)
  (CallFunction|FollowPlayer)
  (Utilities|FlowControl|Delay 0.2))

(event Game|Damage|EventAnyDamage
  (params (Damage :type Float%20%28single-precision%29) (DamageType :type Damage%20Type%20Object%20Reference) (InstigatedBy :type Controller%20Object%20Reference) (DamageCauser :type Actor%20Object%20Reference))
  ;[1 1 1] Take Damage
  (Game|SpawnActorfromClass "/Game/UI/DmgNumbers/BP_DamageNumber.BP_DamageNumber_C" (Math|Transform|MakeTransform (.location (Transformation|GetActorTransform self)) "0, 0, 0" "1.000000,1.000000,1.000000") "Undefined" "MultiplyWithRoot" 0 Damage 0)
  (Variables|Default|SetCurrentEnemyHP (Math|Float|Clamp(Float) (- (Variables|Default|GetCurrentEnemyHP) Damage) 0.0 (Variables|Default|GetMaxEnemyHP)))
  (if (== (Variables|Default|GetCurrentEnemyHP) 0.0)
    (Actor|DestroyActor)
    (bind _astop_down_character_blueprint (Utilities|Casting|CastToTopDownCharacterBlueprint (Game|GetPlayerCharacter 0)))
    (Default|AddEXP _astop_down_character_blueprint 30)))

(fn ConstructionScript)

(fn Shot
  (bind _returnvalue (Game|GetPlayerCharacter 0))
  (bind _self self)
  (bind _self_2 self)
  (bind _returnvalue_2 (Transformation|GetActorLocation _returnvalue))
  (bind _returnvalue_3 (Transformation|GetActorLocation _self_2))
  (bind _returnvalue_4 (Transformation|GetActorTransform _self))
  (bind _returnvalue_5 (- _returnvalue_2 _returnvalue_3))
  (bind _returnvalue_6 (Math|Conversions|RotationFromXVector _returnvalue_5))
  (Game|SpawnActorfromClass "/Game/Character/Weapons/RangedWeapons/BP_Ranged_Weapon_Magic_Enemy1.BP_Ranged_Weapon_Magic_Enemy1_C" (Math|Transform|MakeTransform (Math|Vector|MakeVector (.x (.location _returnvalue_4)) (.y (.location _returnvalue_4)) 0.0) (Math|Rotator|MakeRotator (.roll _returnvalue_6) 0.0 (.yaw _returnvalue_6)) "1.000000,1.000000,1.000000") "AlwaysSpawn" "MultiplyWithRoot" 0 0))