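; Enemy paper character that fires ranged magic at the player on sight and awards EXP when killed.
; A Sphere overlap with TopDownCharacterBlueprint toggles SeesPlayer, which Tick polls through ShotPlayer.
; ShotPlayer spawns BP_Ranged_Weapon_Magic_Enemy facing the player without pitch, using an IsShooting flag and Delay as a cooldown.
; AnyDamage lowers clamped HP, and at zero destroys the enemy and calls AddEXP on the player.
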(event OnComponentBeginOverlap(Sphere)
  (params (OverlappedComponent :type Primitive%20Component%20Object%20Reference) (OtherActor :type Actor%20Object%20Reference) (OtherComp :type Primitive%20Component%20Object%20Reference) (OtherBodyIndex :type Integer) (bFromSweep :type Boolean) (SweepResult :type Hit%20Result%20Structure%20%28by%20ref%29))
  (Utilities|Casting|CastToTopDownCharacterBlueprint OtherActor)
  (Variables|Default|SetseesPlayer true))

(event OnComponentEndOverlap(Sphere)
  (params (OverlappedComponent :type Primitive%20Component%20Object%20Reference) (OtherActor :type Actor%20Object%20Reference) (OtherComp :type Primitive%20Component%20Object%20Reference) (OtherBodyIndex :type Integer))
  (Utilities|Casting|CastToTopDownCharacterBlueprint OtherActor)
  (Variables|Default|SetseesPlayer false))

(event Custom|ShotPlayer
  (bind _returnvalue (Game|GetPlayerCharacter 0))
  (bind _self self)
  (bind _returnvalue_2 (Transformation|GetActorLocation _returnvalue))
  (bind _returnvalue_3 (Transformation|GetActorLocation _self))
  (bind _returnvalue_4 (- _returnvalue_2 _returnvalue_3))
  (bind _returnvalue_5 (Math|Conversions|RotationFromXVector _returnvalue_4))
  (if (and (Variables|Default|GetseesPlayer) (not (Variables|Default|GetisShooting)))
    (Variables|Default|SetisShooting true)
    (Game|SpawnActorfromClass "/Game/Character/Weapons/RangedWeapons/BP_Ranged_Weapon_Magic_Enemy.BP_Ranged_Weapon_Magic_Enemy_C" (Math|Transform|MakeTransform (.location (Transformation|GetActorTransform self)) (Math|Rotator|MakeRotator (.roll _returnvalue_5) 0.0 (.yaw _returnvalue_5)) "1.000000,1.000000,1.000000") "AlwaysSpawn" "MultiplyWithRoot" 0 0)
    (Utilities|FlowControl|Delay 0.5)
    (Variables|Default|SetisShooting false)))

(event EventBeginPlay
  (Variables|Default|SetseesPlayer false)
  (Variables|Default|SetCurrentEnemyHP (Variables|Default|GetMaxEnemyHP)))

(event Collision|EventActorBeginOverlap
  (params (OtherActor :type Actor%20Object%20Reference)))

(event Game|Damage|EventAnyDamage
  (params (Damage :type Float%20%28single-precision%29) (DamageType :type Damage%20Type%20Object%20Reference) (InstigatedBy :type Controller%20Object%20Reference) (DamageCauser :type Actor%20Object%20Reference))
  (Variables|Default|SetCurrentEnemyHP (Math|Float|Clamp(Float) (- (Variables|Default|GetCurrentEnemyHP) Damage) 0.0 (Variables|Default|GetMaxEnemyHP)))
  (if (== (Variables|Default|GetCurrentEnemyHP) 0.0)
    (Actor|DestroyActor)
    (bind _astop_down_character_blueprint (Utilities|Casting|CastToTopDownCharacterBlueprint (Game|GetPlayerCharacter 0)))
    (Default|AddEXP _astop_down_character_blueprint 30)))

(event EventTick
  (params (DeltaSeconds :type Float%20%28single-precision%29))
  (CallFunction|ShotPlayer))

(fn ConstructionScript)