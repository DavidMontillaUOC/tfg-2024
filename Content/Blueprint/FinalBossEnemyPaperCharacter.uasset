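; Final boss Paper character that chases the player inside a detection sphere, with its height locked each tick.
; In close range it stops, and a timeline triggers big-sword attacks, then two-shot magic projectile bursts aimed at the player.
; At half health it enrages, adding a second burst with a shorter cooldown.
; Damage spawns floating numbers; death grants EXP, marks the game finished, pauses and shows the GameFinish screen.
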(event OnComponentBeginOverlap(Sphere)
  (params (OverlappedComponent :type Primitive%20Component%20Object%20Reference) (OtherActor :type Actor%20Object%20Reference) (OtherComp :type Primitive%20Component%20Object%20Reference) (OtherBodyIndex :type Integer) (bFromSweep :type Boolean) (SweepResult :type Hit%20Result%20Structure%20%28by%20ref%29))
  (Utilities|Casting|CastToTopDownCharacterBlueprint OtherActor)
  (Variables|Default|SetseesPlayer true))

(event OnComponentEndOverlap(Sphere)
  (params (OverlappedComponent :type Primitive%20Component%20Object%20Reference) (OtherActor :type Actor%20Object%20Reference) (OtherComp :type Primitive%20Component%20Object%20Reference) (OtherBodyIndex :type Integer))
  (Utilities|Casting|CastToTopDownCharacterBlueprint OtherActor)
  (Variables|Default|SetseesPlayer false))

(event Custom|ShotPlayer
  (if (and (Variables|Default|GetseesPlayer) (not (Variables|Default|GetisShooting)))
    (Variables|Default|SetisShooting true)
    (|RapidFire_2)
    (Variables|Default|SetisShooting false)
    (if (Variables|Default|Getenrage)
      (Variables|Default|SetisShooting true)
      (|RapidFire_2_2)
      (Utilities|FlowControl|Delay 1.5)
      (Variables|Default|SetisShooting false)
      (else
        (Utilities|FlowControl|Delay 2.0)
        (Variables|Default|SetisShooting false)))))

(event Custom|FollowPlayer
  (bind (_returnvalue_x _returnvalue_y) (|ReturnPlayerDirection))
  (bind _charactermovement (Variables|Character|GetCharacterMovement))
  ;[1 1 1] Track Player
  (if (Variables|Default|GetseesPlayer)
    (if (> (Math|Vector|VectorLength (Math|Vector|MakeVector _returnvalue_x _returnvalue_y 0.0)) 3e+02)
      (Pawn|Components|CharacterMovement|SetMovementMode _charactermovement "MOVE_Walking" 0)
      (Pawn|Input|AddMovementInput (Math|Vector|MakeVector _returnvalue_x 0.0 0.0) 1.0 false)
      (Pawn|Input|AddMovementInput (Math|Vector|MakeVector 0.0 _returnvalue_y 0.0) 1.0 false)
      (Variables|Default|SetDirection (Math|Vector2D|MakeVector2D _returnvalue_x _returnvalue_y))
      (Variables|Default|SetcanAttack false)
      (else
        (Pawn|Components|CharacterMovement|DisableMovement _charactermovement)
        (Variables|Default|SetcanAttack true)))))

(event Custom|attackPlayer
  (bind _returnvalue (Game|GetPlayerCharacter 0))
  (bind _returnvalue_2 (Transformation|GetActorLocation))
  (bind _returnvalue_3 (Transformation|GetActorLocation _returnvalue))
  (bind _returnvalue_4 (- _returnvalue_3 _returnvalue_2))
  ;[1 1 1] Attack Player
  (Variables|Default|SetisAttacking true)
  (Utilities|FlowControl|Delay 1.0)
  (Variables|Default|SetisAttacking false)
  (Game|SpawnActorfromClass "/Game/Character/Weapons/Melee/BP_AnimationBigSwordEnemy.BP_AnimationBigSwordEnemy_C" (Math|Transform|MakeTransform (.location (Transformation|GetActorTransform)) (Math|Rotator|MakeRotator 0.0 0.0 (- (Class|KismetMathLibrary|DegAtan2 (.y _returnvalue_4) (.x _returnvalue_4)) 180)) "2.000000,2.000000,2.000000") "Undefined" "MultiplyWithRoot" 0 0))

(event EventBeginPlay
  (Variables|Default|SetseesPlayer false)
  (Variables|Default|SetCurrentEnemyHP (Variables|Default|GetMaxEnemyHP)))

(event Collision|EventActorBeginOverlap
  (params (OtherActor :type Actor%20Object%20Reference)))

(event EventTick
  (params (DeltaSeconds :type Float%20%28single-precision%29))
  (bind _self self)
  (bind _returnvalue (Transformation|GetActorLocation _self))
  (Transformation|SetActorLocation (Math|Vector|MakeVector (.x _returnvalue) (.y _returnvalue) 159.513458) false false)
  (if (<= (Variables|Default|GetCurrentEnemyHP) (/ (Variables|Default|GetMaxEnemyHP) 2))
    (Variables|Default|Setenrage true))
  (if (Variables|Default|GetseesPlayer)
    (CallFunction|FollowPlayer)
    (if (and (Variables|Default|GetcanAttack) (not (Variables|Default|GetisAttacking)))
      (Utilities|FlowControl|Delay 0.2)
      (Timeline|Timeline Play
        (:Update
          (CallFunction|AttackPlayer))
        (:Finished
          (CallFunction|ShotPlayer))))))

(event Game|Damage|EventAnyDamage
  (params (Damage :type Float%20%28single-precision%29) (DamageType :type Damage%20Type%20Object%20Reference) (InstigatedBy :type Controller%20Object%20Reference) (DamageCauser :type Actor%20Object%20Reference))
  (bind _returnvalue (Game|GetPlayerController 0))
  ;[1 1 1] Take Damage
  (Game|SpawnActorfromClass "/Game/UI/DmgNumbers/BP_DamageNumber.BP_DamageNumber_C" (Math|Transform|MakeTransform (.location (Transformation|GetActorTransform self)) "0, 0, 0" "1.000000,1.000000,1.000000") "Undefined" "MultiplyWithRoot" 0 Damage 0)
  (Variables|Default|SetCurrentEnemyHP (Math|Float|Clamp(Float) (- (Variables|Default|GetCurrentEnemyHP) Damage) 0.0 (Variables|Default|GetMaxEnemyHP)))
  (if (== (Variables|Default|GetCurrentEnemyHP) 0.0)
    (bind _astop_down_character_blueprint (Utilities|Casting|CastToTopDownCharacterBlueprint (Game|GetPlayerCharacter 0)))
    (Default|AddEXP _astop_down_character_blueprint 30)
    (Default|SetGameFinished _astop_down_character_blueprint)
    (Utilities|FlowControl|Delay 0.2)
    (Game|SetGamePaused true)
    (bind _returnvalue_2 (UserInterface|CreateWidget "/Game/UI/GameFinish.GameFinish_C"))
    (UserInterface|Viewport|AddtoViewport _returnvalue_2 0)
    (Variables|/Script/Engine.PlayerController|SetbShowMouseCursor _returnvalue true)
    (Input|SetInputModeUIOnly _returnvalue _returnvalue_2 "DoNotLock" false)
    (Actor|DestroyActor)))

(fn ConstructionScript)

(fn Shot
  (bind _returnvalue (Game|GetPlayerCharacter 0))
  (bind _self self)
  (bind _self_2 self)
  (bind _returnvalue_2 (Transformation|GetActorLocation _returnvalue))
  (bind _returnvalue_3 (Transformation|GetActorLocation _self_2))
  (bind _returnvalue_4 (Transformation|GetActorTransform _self))
  (bind _returnvalue_5 (- _returnvalue_2 _returnvalue_3))
  (bind _returnvalue_6 (Math|Conversions|RotationFromXVector (Math|Vector|MakeVector (.x _returnvalue_5) (.y _returnvalue_5) (.z _returnvalue_5))))
  (bind _returnvalue_7 (* (.y _returnvalue_5) 1.05))
  (bind _returnvalue_8 (* (.x _returnvalue_5) 1.05))
  (bind _returnvalue_9 (Math|Vector|Normalize (Math|Vector|MakeVector _returnvalue_8 _returnvalue_7 0.0)))
  (Game|SpawnActorfromClass "/Game/Character/Weapons/RangedWeapons/BP_Ranged_Weapon_Magic_Enemy1.BP_Ranged_Weapon_Magic_Enemy1_C" (Math|Transform|MakeTransform (Math|Vector|MakeVector (+ (.x (.location _returnvalue_4)) (.x _returnvalue_9)) (+ (.y (.location _returnvalue_4)) (.y _returnvalue_9)) 0.0) (Math|Rotator|MakeRotator (.roll _returnvalue_6) 0.0 (.yaw _returnvalue_6)) "1.000000,1.000000,1.000000") "AlwaysSpawn" "MultiplyWithRoot" 0 0))