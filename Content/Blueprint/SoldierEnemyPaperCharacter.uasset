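; Melee soldier enemy character that chases and attacks the top-down player and awards EXP on death.
; A detection sphere sets SeesPlayer, and Tick drives pursuit until close range, where movement stops and delayed attacks spawn a sword-swing actor rotated toward the player.
; Losing sight switches movement to Flying, then disables it after a delay.
; Damage spawns floating numbers and reduces clamped HP, destroying the enemy at zero.
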(event OnComponentBeginOverlap(Sphere)
  (params (OverlappedComponent :type Primitive%20Component%20Object%20Reference) (OtherActor :type Actor%20Object%20Reference) (OtherComp :type Primitive%20Component%20Object%20Reference) (OtherBodyIndex :type Integer) (bFromSweep :type Boolean) (SweepResult :type Hit%20Result%20Structure%20%28by%20ref%29))
  (Utilities|Casting|CastToTopDownCharacterBlueprint OtherActor)
  (Variables|Default|SetseesPlayer true))

(event OnComponentEndOverlap(Sphere)
  (params (OverlappedComponent :type Primitive%20Component%20Object%20Reference) (OtherActor :type Actor%20Object%20Reference) (OtherComp :type Primitive%20Component%20Object%20Reference) (OtherBodyIndex :type Integer))
  (Utilities|Casting|CastToTopDownCharacterBlueprint OtherActor)
  (Variables|Default|SetseesPlayer false))

(event Custom|FollowPlayer
  (bind (_returnvalue_x _returnvalue_y) (|ReturnPlayerDirection))
  (bind _charactermovement (Variables|Character|GetCharacterMovement))
  ;[1 1 1] Track Player
  (if (Variables|Default|GetseesPlayer)
    (if (> (Math|Vector|VectorLength (Math|Vector|MakeVector _returnvalue_x _returnvalue_y 0.0)) 1.2e+02)
      (Pawn|Components|CharacterMovement|SetMovementMode _charactermovement "MOVE_Walking" 0)
      (Pawn|Input|AddMovementInput (Math|Vector|MakeVector _returnvalue_x 0.0 0.0) 1.0 false)
      (Pawn|Input|AddMovementInput (Math|Vector|MakeVector 0.0 _returnvalue_y 0.0) 1.0 false)
      (Variables|Default|SetDirection (Math|Vector2D|MakeVector2D _returnvalue_x _returnvalue_y))
      (Variables|Default|SetcanAttack false)
      (else
        (Pawn|Components|CharacterMovement|DisableMovement _charactermovement)
        (Variables|Default|SetcanAttack true)))))

(event Custom|attackPlayer
  (bind _returnvalue (Game|GetPlayerCharacter 0))
  (bind _returnvalue_2 (Transformation|GetActorLocation))
  (bind _returnvalue_3 (Transformation|GetActorLocation _returnvalue))
  (bind _returnvalue_4 (- _returnvalue_3 _returnvalue_2))
  ;[1 1 1] Attack Player
  (Variables|Default|SetisAttacking true)
  (Utilities|FlowControl|Delay 1.0)
  (Variables|Default|SetisAttacking false)
  (Game|SpawnActorfromClass "/Game/Character/Weapons/Melee/BP_AnimationBigSwordEnemy.BP_AnimationBigSwordEnemy_C" (Math|Transform|MakeTransform (.location (Transformation|GetActorTransform)) (Math|Rotator|MakeRotator 0.0 0.0 (- (Class|KismetMathLibrary|DegAtan2 (.y _returnvalue_4) (.x _returnvalue_4)) 180)) "1.000000,1.000000,1.000000") "Undefined" "MultiplyWithRoot" 0 0))

(event EventBeginPlay
  (Variables|Default|SetseesPlayer false)
  (Variables|Default|SetCurrentEnemyHP (Variables|Default|GetMaxEnemyHP)))

(event Collision|EventActorBeginOverlap
  (params (OtherActor :type Actor%20Object%20Reference)))

(event EventTick
  (params (DeltaSeconds :type Float%20%28single-precision%29))
  (bind _charactermovement (Variables|Character|GetCharacterMovement))
  (if (Variables|Default|GetseesPlayer)
    (CallFunction|FollowPlayer)
    (if (and (Variables|Default|GetcanAttack) (not (Variables|Default|GetisAttacking)))
      (Utilities|FlowControl|Delay 0.2)
      (CallFunction|AttackPlayer))
    (else
      (Pawn|Components|CharacterMovement|SetMovementMode _charactermovement "MOVE_Flying" 0)
      (Class|CharacterMovementComponent|CalcVelocity _charactermovement 0.0 0.1 false 0.1)
      (Utilities|FlowControl|Delay 2.0)
      (Pawn|Components|CharacterMovement|DisableMovement _charactermovement))))

(event Game|Damage|EventAnyDamage
  (params (Damage :type Float%20%28single-precision%29) (DamageType :type Damage%20Type%20Object%20Reference) (InstigatedBy :type Controller%20Object%20Reference) (DamageCauser :type Actor%20Object%20Reference))
  ;[1 1 1] Take Damage
  (Game|SpawnActorfromClass "/Game/UI/DmgNumbers/BP_DamageNumber.BP_DamageNumber_C" (Math|Transform|MakeTransform (.location (Transformation|GetActorTransform self)) "0, 0, 0" "1.000000,1.000000,1.000000") "Undefined" "MultiplyWithRoot" 0 Damage 0)
  (Variables|Default|SetCurrentEnemyHP (Math|Float|Clamp(Float) (- (Variables|Default|GetCurrentEnemyHP) Damage) 0.0 (Variables|Default|GetMaxEnemyHP)))
  (if (== (Variables|Default|GetCurrentEnemyHP) 0.0)
    (Actor|DestroyActor)
    (bind _astop_down_character_blueprint (Utilities|Casting|CastToTopDownCharacterBlueprint (Game|GetPlayerCharacter 0)))
    (Default|AddEXP _astop_down_character_blueprint 30)))

(fn ConstructionScript)