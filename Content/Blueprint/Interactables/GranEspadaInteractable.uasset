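; Interactable actor for a great sword that shows an on-screen widget while something is inside its box trigger.
; Box begin and end overlap toggle the widget's visibility without filtering the overlapping actor, and print debug strings.
; The BeginInteraction event calls the parent implementation and prints a placeholder message, with no pickup or other gameplay logic yet.
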(event OnComponentBeginOverlap(Box)
  (params (OverlappedComponent :type Primitive%20Component%20Object%20Reference) (OtherActor :type Actor%20Object%20Reference) (OtherComp :type Primitive%20Component%20Object%20Reference) (OtherBodyIndex :type Integer) (bFromSweep :type Boolean) (SweepResult :type Hit%20Result%20Structure%20%28by%20ref%29))
  (Rendering|SetVisibility (Variables|Default|GetWidget) true false)
  (Development|PrintString "Si GramEspada"))

(event OnComponentEndOverlap(Box)
  (params (OverlappedComponent :type Primitive%20Component%20Object%20Reference) (OtherActor :type Actor%20Object%20Reference) (OtherComp :type Primitive%20Component%20Object%20Reference) (OtherBodyIndex :type Integer))
  (Rendering|SetVisibility (Variables|Default|GetWidget) false false)
  (Development|PrintString "No GranEspada"))

(event EventBeginInteraction
  (|CallParentFunction)
  (Development|PrintString "Henlo"))

(fn ConstructionScript
  (|CallParentFunction))