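; Trigger actor that shows the mage boss's health bar while the player is inside its box.
; BeginPlay finds the first actor tagged "boss1" and stores it as Boss after a short delay.
; Player overlap creates a BossHp widget on the viewport, and end overlap removes it.
; Tick pushes the boss's current and max HP to the widget and destroys this trigger actor when HP equals zero.
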(event OnComponentBeginOverlap(Box)
  (params (OverlappedComponent :type Primitive%20Component%20Object%20Reference) (OtherActor :type Actor%20Object%20Reference) (OtherComp :type Primitive%20Component%20Object%20Reference) (OtherBodyIndex :type Integer) (bFromSweep :type Boolean) (SweepResult :type Hit%20Result%20Structure%20%28by%20ref%29))
  (bind _boss (Variables|Default|Getboss))
  (if (== OtherActor (Game|Player|GetPlayerPawn 0))
    (bind _returnvalue (UserInterface|CreateWidget "/Game/UI/BossHp.BossHp_C"))
    (UserInterface|Viewport|AddtoViewport _returnvalue 0)
    (bind _output_get (Variables|Default|SetwidgetHP _returnvalue))
    (bind _asboss_hp (Utilities|Casting|CastToBossHp _output_get))
    (Default|SetHPBar _asboss_hp (Variables|/Game/Blueprint/MageBossEnemyPaperCharacter.MageBossEnemyPaperCharacter_C|GetCurrentEnemyHP _boss) (Variables|/Game/Blueprint/MageBossEnemyPaperCharacter.MageBossEnemyPaperCharacter_C|GetMaxEnemyHP _boss))))

(event OnComponentEndOverlap(Box)
  (params (OverlappedComponent :type Primitive%20Component%20Object%20Reference) (OtherActor :type Actor%20Object%20Reference) (OtherComp :type Primitive%20Component%20Object%20Reference) (OtherBodyIndex :type Integer))
  (if (== OtherActor (Game|Player|GetPlayerPawn 0))
    (Widget|RemovefromParent (Variables|Default|GetwidgetHP))))

(event EventBeginPlay
  (bind _outactors (Actor|GetAllActorswithTag "boss1"))
  (bind _asmage_boss_enemy_paper_character (Utilities|Casting|CastToMageBossEnemyPaperCharacter (Utilities|Array|Get(acopy) _outactors)))
  (Utilities|FlowControl|Delay 0.5)
  (Variables|Default|Setboss _asmage_boss_enemy_paper_character))

(event Collision|EventActorBeginOverlap
  (params (OtherActor :type Actor%20Object%20Reference)))

(event EventTick
  (params (DeltaSeconds :type Float%20%28single-precision%29))
  (bind _boss (Variables|Default|Getboss))
  (bind _asboss_hp (Utilities|Casting|CastToBossHp (Variables|Default|GetwidgetHP)))
  (Default|SetHPBar _asboss_hp (Variables|/Game/Blueprint/MageBossEnemyPaperCharacter.MageBossEnemyPaperCharacter_C|GetCurrentEnemyHP _boss) (Variables|/Game/Blueprint/MageBossEnemyPaperCharacter.MageBossEnemyPaperCharacter_C|GetMaxEnemyHP _boss))
  (if (== (Variables|/Game/Blueprint/MageBossEnemyPaperCharacter.MageBossEnemyPaperCharacter_C|GetCurrentEnemyHP (Variables|Default|Getboss)) 0.0)
    (Actor|DestroyActor)))

(fn ConstructionScript
  (|CallParentFunction))