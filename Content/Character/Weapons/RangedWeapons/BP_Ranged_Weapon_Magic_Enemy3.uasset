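; BP_Ranged_Weapon_Magic_Enemy3 is an enemy magic projectile that damages the top-down player character on overlap.
; BeginPlay adds a ProjectileMovement component at runtime and gives it a fixed speed.
; Overlapping the player prints a debug string, applies fixed damage unless the player is invincible, and destroys the projectile either way.
; Tick only runs a Delay with nothing after it, so the projectile has no timed self-destruct.
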(event EventBeginPlay
  (bind _returnvalue (AddComponent|AddProjectileMovementComponent))
  (Variables|/Script/Engine.ProjectileMovementComponent|SetInitialSpeed _returnvalue 3e+02)
  (Variables|/Script/Engine.ProjectileMovementComponent|SetMaxSpeed _returnvalue 3e+02))

(event Collision|EventActorBeginOverlap
  (params (OtherActor :type Actor%20Object%20Reference))
  (bind _astop_down_character_blueprint (Utilities|Casting|CastToTopDownCharacterBlueprint OtherActor))
  (Development|PrintString "coño")
  (if (not (Variables|/Game/Blueprint/TopDownCharacterBlueprint.TopDownCharacterBlueprint_C|GetplayerInvincible _astop_down_character_blueprint))
    (Game|Damage|ApplyDamage _astop_down_character_blueprint 1e+01 0 0)
    (Actor|DestroyActor)
    (else
      (Actor|DestroyActor))))

(event EventTick
  (params (DeltaSeconds :type Float%20%28single-precision%29))
  (Utilities|FlowControl|Delay 2.0))

(fn ConstructionScript)