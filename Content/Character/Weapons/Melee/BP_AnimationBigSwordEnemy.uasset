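; BP_AnimationBigSwordEnemy is a short-lived melee attack actor, named for an enemy's big sword swing, that can hurt the player.
; A non-looping PaperFlipbook plays the animation, and the actor destroys itself when it finishes.
; While it exists, HitBox overlaps with actors whose root is tagged "player" apply fixed damage to the player pawn, unless the TopDownCharacterBlueprint is flagged invincible.
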(event OnFinishedPlaying(PaperFlipbook)
  (Actor|DestroyActor))

(event OnComponentBeginOverlap(HitBox)
  (params (OverlappedComponent :type Primitive%20Component%20Object%20Reference) (OtherActor :type Actor%20Object%20Reference) (OtherComp :type Primitive%20Component%20Object%20Reference) (OtherBodyIndex :type Integer) (bFromSweep :type Boolean) (SweepResult :type Hit%20Result%20Structure%20%28by%20ref%29))
  (bind _returnvalue (Game|Player|GetPlayerPawn 0))
  (bind _astop_down_character_blueprint (Utilities|Casting|CastToTopDownCharacterBlueprint _returnvalue))
  (if (and (not (Variables|/Game/Blueprint/TopDownCharacterBlueprint.TopDownCharacterBlueprint_C|GetplayerInvincible _astop_down_character_blueprint)) (Components|ComponentHasTag (Variables|/Script/Engine.Actor|GetRootComponent OtherActor) "player"))
    (Game|Damage|ApplyDamage _returnvalue 2e+01 0 0 "/Script/Engine.DamageType")))

(event OnComponentHit(HitBox)
  (params (HitComponent :type Primitive%20Component%20Object%20Reference) (OtherActor :type Actor%20Object%20Reference) (OtherComp :type Primitive%20Component%20Object%20Reference) (NormalImpulse :type Vector :default "0, 0, 0") (Hit :type Hit%20Result%20Structure%20%28by%20ref%29)))

(event EventBeginPlay
  (Components|Timeline|SetLooping (Variables|Default|GetPaperFlipbook) false))

(event EventTick
  (params (DeltaSeconds :type Float%20%28single-precision%29)))

(fn ConstructionScript)