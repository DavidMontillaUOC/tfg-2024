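; BP_AnimationSpear is a short-lived spear attack actor that plays a non-looping Paper2D flipbook and destroys itself when playback finishes.
; When its HitBox overlaps a component tagged enemyCollider, it applies damage to that component's owning actor.
; Damage is a flat base plus a Scaling value from the AScalingDT data table, using the player character's Agilidad stat as the row name.
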(event OnFinishedPlaying(PaperFlipbook)
  (Actor|DestroyActor))

(event OnComponentBeginOverlap(HitBox)
  (params (OverlappedComponent :type Primitive%20Component%20Object%20Reference) (OtherActor :type Actor%20Object%20Reference) (OtherComp :type Primitive%20Component%20Object%20Reference) (OtherBodyIndex :type Integer) (bFromSweep :type Boolean) (SweepResult :type Hit%20Result%20Structure%20%28by%20ref%29))
  (bind _astop_down_character_blueprint (Utilities|Casting|CastToTopDownCharacterBlueprint (Game|Player|GetPlayerPawn 0)))
  (bind _returnvalue (Utilities|GetDataTableRow "/Game/Config/A-Scaling-DT.A-Scaling-DT" (Utilities|String|StringToName (Utilities|String|ToString(Integer) (Variables|/Game/Blueprint/TopDownCharacterBlueprint.TopDownCharacterBlueprint_C|GetAgilidad _astop_down_character_blueprint))))
    (:then
      (if (Components|ComponentHasTag OtherComp "enemyCollider")
        (Game|Damage|ApplyDamage OtherActor (+ (.Scaling (Utilities|Struct|BreakAttributeScalingStruct _returnvalue)) 12.0) 0 0)))))

(event EventBeginPlay
  (Components|Timeline|SetLooping (Variables|Default|GetPaperFlipbook) false))

(event Collision|EventActorBeginOverlap
  (params (OtherActor :type Actor%20Object%20Reference)))

(event EventTick
  (params (DeltaSeconds :type Float%20%28single-precision%29)))

(fn ConstructionScript)