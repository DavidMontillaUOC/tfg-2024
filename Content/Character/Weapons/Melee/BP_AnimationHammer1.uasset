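; BP_AnimationHammer1 is a short-lived hammer melee attack actor that plays its flipbook animation once and destroys itself when playback finishes.
; Its HitBox overlap damages an EnemyPaperCharacter when the touched component carries the enemyCollider tag, scaling damage from the player character's Fuerza stat plus a flat bonus.
; Each hit also prints a long-lasting debug message.
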(event OnFinishedPlaying(PaperFlipbook)
  (Actor|DestroyActor))

(event OnComponentBeginOverlap(HitBox)
  (params (OverlappedComponent :type Primitive%20Component%20Object%20Reference) (OtherActor :type Actor%20Object%20Reference) (OtherComp :type Primitive%20Component%20Object%20Reference) (OtherBodyIndex :type Integer) (bFromSweep :type Boolean) (SweepResult :type Hit%20Result%20Structure%20%28by%20ref%29))
  (bind _astop_down_character_blueprint (Utilities|Casting|CastToTopDownCharacterBlueprint (Game|Player|GetPlayerPawn 0)))
  (bind _asenemy_paper_character (Utilities|Casting|CastToEnemyPaperCharacter OtherActor))
  (if (Components|ComponentHasTag OtherComp "enemyCollider")
    (Game|Damage|ApplyDamage _asenemy_paper_character (+ (* (Variables|/Game/Blueprint/TopDownCharacterBlueprint.TopDownCharacterBlueprint_C|GetFuerza _astop_down_character_blueprint) 1.5) 3e+01) 0 0)
    (Development|PrintString "dmg done" true true "(R=0.000000,G=0.660000,B=1.000000,A=1.000000)" 5e+02)))

(event EventBeginPlay
  (Components|Timeline|SetLooping (Variables|Default|GetPaperFlipbook) false))

(event Collision|EventActorBeginOverlap
  (params (OtherActor :type Actor%20Object%20Reference)))

(event EventTick
  (params (DeltaSeconds :type Float%20%28single-precision%29)))

(fn ConstructionScript)